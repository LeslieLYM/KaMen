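; Player controller that handles switching the controlled pawn through a Kamen mask system.
; Its construction script registers the mask master component, and the Equip_1 input requests a pawn switch at the current pawn's transform, then has that component check mask 1.
; One second after BeginPlay, it destroys the Kamen and Puppet pawns returned by its getters.
; The switch logic itself is defined outside these graphs.
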(event EventBeginPlay
  (Utilities|FlowControl|Delay 1.0)
  (bind _returnvalue (Class|MainPlayerController|GetKamenPawn))
  (Actor|DestroyActor _returnvalue)
  (bind _returnvalue_2 (Class|MainPlayerController|GetPuppetPawn))
  (Actor|DestroyActor _returnvalue_2))

(event EventTick
  (params (DeltaSeconds :type Float%20%28single-precision%29)))

(event Input|ActionEvents|InputActionChangePosses
  (params (Key :type Key%20Structure)))

(event Input|ActionEvents|InputActionEquip_1
  (params (Key :type Key%20Structure))
  (bind _returnvalue (Pawn|GetControlledPawn))
  (:Pressed
    (Class|MainPlayerController|IntendSwitchPawn _returnvalue (Transformation|GetActorTransform _returnvalue))
    (Class|KaMenMaskMasterComponent|CheckMask (Variables|Default|GetKaMenMaskMasterComponent_C) 1)))

(fn ConstructionScript
  (Class|MainPlayerController|SetMaskMasterReference (Variables|Default|GetKaMenMaskMasterComponent_C)))