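; KaMenPawn_BP is a player-controlled KaMen pawn that moves sideways, jumps and uses masks.
; Input events forward the right axis and jump to IntendRight and IntendJump, and Equip_1 asks the mask master component to check mask 1.
; The construction script sizes the capsule collider from variables and hands the body and mask meshes to the pawn and mask component.
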(event EventBeginPlay)

(event Collision|EventActorBeginOverlap
  (params (OtherActor :type Actor%20Object%20Reference)))

(event EventTick
  (params (DeltaSeconds :type Float%20%28single-precision%29)))

(event Input|ActionEvents|InputActionJump
  (params (Key :type Key%20Structure))
  (:Pressed
    (Class|KaMenPawn|IntendJump)))

(event Input|ActionEvents|InputActionEquip_1
  (params (Key :type Key%20Structure))
  (:Pressed
    (Class|KaMenMaskMasterComponent|CheckMask (Variables|Default|GetKaMenMaskMasterComponent_C) Key 1)))

(event Input|AxisEvents|InputAxisIntendRight
  (params (AxisValue :type Float%20%28single-precision%29))
  (Class|KaMenPawn|IntendRight AxisValue))

(fn ConstructionScript
  (bind _overallcollider (Variables|Default|GetOverallCollider))
  (Components|Capsule|SetCapsuleHalfHeight _overallcollider (Variables|SetUp|GetCapsuleHeight) true)
  (Components|Capsule|SetCapsuleRadius _overallcollider (Variables|SetUp|GetCapsuleRadius) true)
  (Class|KaMenPawn|SetKamenMeshReference (Variables|Default|GetKaMen))
  (Class|KaMenPawn|SetKamenMaskMeshReference (Variables|Default|GetKaMenMaskStaticMeshComponent_C))
  (Class|KaMenMaskMasterComponent|SetMaskStaticMeshReference (Variables|Default|GetKaMenMaskMasterComponent_C) (Variables|Default|GetKaMenMaskStaticMeshComponent_C) (Variables|Default|GetKaMen)))