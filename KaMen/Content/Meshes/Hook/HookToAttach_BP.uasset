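; Hook actor that takes player input to move sideways and to release an attached player pawn.
; Horizontal input drives the Y physics velocity of Sphere1, whose radius the construction script sets from DetectVolumeRadius, and prints the axis value.
; Downward input detaches the pawn, re-enables gravity on the PuppetPawn_BP capsule and hands input from the hook back to the pawn.
; The attach logic is not in this graph.
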(event EventBeginPlay)

(event Collision|EventActorBeginOverlap
  (params (OtherActor :type Actor%20Object%20Reference)))

(event EventTick
  (params (DeltaSeconds :type Float%20%28single-precision%29)))

(event Input|AxisEvents|InputAxisIntendRight
  (params (AxisValue :type Float%20%28single-precision%29))
  (Development|PrintString (Utilities|String|ToString(Float) AxisValue))
  (Class|PrimitiveComponent|SetAllPhysicsLinearVelocity (Variables|Default|GetSphere1) (Math|Vector|MakeVector 0.0 (* AxisValue 1e+03) 0.0) false))

(event Input|AxisEvents|InputAxisIntendUp
  (params (AxisValue :type Float%20%28single-precision%29))
  (bind _returnvalue (Game|Player|GetPlayerPawn 0))
  (bind _returnvalue_2 (Game|GetPlayerController 0))
  (if (< AxisValue 0.0)
    (Transformation|DetachFromActor _returnvalue "KeepWorld" "KeepWorld" "KeepWorld")
    (bind _aspuppet_pawn_bp (Utilities|Casting|CastToPuppetPawn_BP _returnvalue))
    (Physics|SetEnableGravity (Variables|/Game/Meshes/Puppet/PuppetPawn_BP.PuppetPawn_BP_C|GetCapsule _aspuppet_pawn_bp) true)
    (Input|DisableInput _returnvalue_2)
    (Input|EnableInput _aspuppet_pawn_bp _returnvalue_2)))

(fn ConstructionScript
  (Components|Sphere|SetSphereRadius (Variables|Default|GetSphere1) (Variables|SetUp|GetDetectVolumeRadius) true))